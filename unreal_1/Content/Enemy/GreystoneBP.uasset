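; Greystone enemy Blueprint that wanders, chases the player on sight and attacks in melee.
; BeginPlay links itself to its nameplate health bar.
; Pawn sensing starts an AI move toward the player and sets chase flags; a retriggerable delay clears only CanSeePlayer.
; Tick drives random roaming while not chasing, and player overlap with AttackSphere spawns a sword particle and calls MainMeleeAttack.
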(event `self.ReceiveBeginPlay`
  (bind _asenemy_health_bar (cast `/Game/_Project_1/HUD/EnemyHealthBar` (`WidgetComponent.GetUserWidgetObject` (`self.NamePlate`))))
  (set `/Game/_Project_1/HUD/EnemyHealthBar.Enemy` self _asenemy_health_bar)
  (`Widget.SetVisibility` (`WidgetComponent.GetUserWidgetObject` (`self.NamePlate`)) "Visible"))

(event `self.PawnSensing.OnSeePawn`
  (params (Pawn :type "Pawn Object Reference"))
  ;[1 1 1] Refactor into C++ and Behavior Tree
  (bind _asfinal_player_character (cast `/Game/_Project_1/PlayerCharacter/FinalPlayerCharacter` Pawn))
  (`|ExecutionSequence`
    (:`then_0`
      (set `self.CanSeePlayer` true)
      (set `self.ChasingPlayer` true)
      (`|AIMoveTo` self (0.0 0.0 0.0) _asfinal_player_character))
    (:`then_1`
      (`KismetSystemLibrary.RetriggerableDelay` 0.6)
      (set `self.CanSeePlayer` false))))

(event `self.ReceiveTick`
  (params (DeltaSeconds :type "Float (single-precision)"))
  ;[1 1 1] Refactor into C++ and Behavior Tree
  (if (not (`self.ChasingPlayer`))
    (`KismetSystemLibrary.Delay` (`KismetMathLibrary.RandomFloatInRange` 1.0 5.0))
    (`|AIMoveTo` self (`NavigationSystemV1.K2_GetRandomReachablePointInRadius` (`self.K2_GetActorLocation`) 1000.0 null null) null)))

(event `self.AttackSphere.OnComponentBeginOverlap`
  (params (OverlappedComponent :type "PrimitiveComponent Object Reference") (OtherActor :type "Actor Object Reference") (OtherComp :type "PrimitiveComponent Object Reference") (OtherBodyIndex :type Integer) (bFromSweep :type Boolean) (SweepResult :type "HitResult Structure (by ref)"))
  ;[1 1 1] Refactor into C++ and Behavior Tree
  (cast `/Game/_Project_1/PlayerCharacter/FinalPlayerCharacter` OtherActor)
  (if true
    (`NiagaraFunctionLibrary.SpawnSystemAtLocation` "/Game/Tutorial/Particle/01/Swing_Particle_01.Swing_Particle_01" (.location (`SkinnedMeshComponent.GetBoneTransform` (`self.Mesh`) "sword_top" "RTS_Actor")) (.rotation (`SkinnedMeshComponent.GetBoneTransform` (`self.Mesh`) "sword_top" "RTS_Actor")) (100.0 100.0 100.0) false)
    (`self.MainMeleeAttack`)))

(fn `UserConstructionScript`)