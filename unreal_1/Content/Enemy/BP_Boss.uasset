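; Boss enemy pawn that wanders until it spots the player, then chases and melee attacks.
; While not chasing, Tick uses a random 1–5 second Delay before moving to a random reachable point nearby.
; PawnSensing sightings start an AI move toward the player; a retriggerable delay clears CanSeePlayer, while ChasingPlayer stays set.
; AttackSphere overlaps with actors implementing PlayerCharacterInterface call MainMeleeAttack.
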(event `self.PawnSensing.OnSeePawn`
  (params (Pawn :type "Pawn Object Reference"))
  ;[1 1 1] REFO
  (bind _asplayer_character_bp (cast `/Game/_Project_1/PlayerCharacter/PlayerCharacterBP` Pawn))
  (`|ExecutionSequence`
    (:`then_0`
      (set `self.CanSeePlayer` true)
      (set `self.ChasingPlayer` true)
      (`|AIMoveTo` self (0.0 0.0 0.0) _asplayer_character_bp))
    (:`then_1`
      (`KismetSystemLibrary.RetriggerableDelay` 0.5)
      (set `self.CanSeePlayer` false))))

(event `self.ReceiveTick`
  (params (DeltaSeconds :type "Float (single-precision)"))
  ;[1 1 1] REFO
  (if (not (`self.ChasingPlayer`))
    (`KismetSystemLibrary.Delay` (`KismetMathLibrary.RandomFloatInRange` 1.0 5.0))
    (`|AIMoveTo` self (`NavigationSystemV1.K2_GetRandomReachablePointInRadius` (`self.K2_GetActorLocation`) 1000.0 null null) null)))

(event `self.AttackSphere.OnComponentBeginOverlap`
  (params (OverlappedComponent :type "PrimitiveComponent Object Reference") (OtherActor :type "Actor Object Reference") (OtherComp :type "PrimitiveComponent Object Reference") (OtherBodyIndex :type Integer) (bFromSweep :type Boolean) (SweepResult :type "HitResult Structure (by ref)"))
  ;[1 1 1] REFO
  (if (`KismetSystemLibrary.DoesImplementInterface` OtherActor "/Script/unreal_1.PlayerCharacterInterface")
    (`self.MainMeleeAttack`)))

(fn `UserConstructionScript`)