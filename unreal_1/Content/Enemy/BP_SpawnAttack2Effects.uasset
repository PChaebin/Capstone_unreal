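; Anim notify that spawns particle effects for an enemy's second attack.
; When fired, it spawns a swing effect at the mesh's sword_top socket, matching its world location and rotation, and prints a debug string.
; It then spawns a second effect at the owner's forward vector multiplied by its location, a component-wise product rather than an offset in front of the owner.
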(fn `Received_Notify`
  (params (MeshComp :type "SkeletalMeshComponent Object Reference") (Animation :type "AnimSequenceBase Object Reference") (EventReference :type "AnimNotifyEventReference Structure (by ref)"))
  (returns (ReturnValue :type Boolean))
  (bind _returnvalue (`ActorComponent.GetOwner` MeshComp))
  (`NiagaraFunctionLibrary.SpawnSystemAtLocation` "/Game/Tutorial/Particle/01/Swing_Particle_01.Swing_Particle_01" (.location (`SceneComponent.GetSocketTransform` MeshComp "sword_top" "RTS_World")) (.rotation (`SceneComponent.GetSocketTransform` MeshComp "sword_top" "RTS_World")))
  (`KismetSystemLibrary.PrintString` "Hello")
  (`NiagaraFunctionLibrary.SpawnSystemAtLocation` "/Game/Tutorial/Particle/02/Exp_01.Exp_01" (* (`Actor.GetActorForwardVector` _returnvalue) (`Actor.K2_GetActorLocation` _returnvalue)))
  (return true))